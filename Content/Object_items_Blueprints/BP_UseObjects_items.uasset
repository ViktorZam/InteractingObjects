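; Usable item actor that labels itself through a widget component showing its name and description.
; On BeginPlay it writes NameObject and DescriptionObject into its W_Object_items widget, replacing the #N# placeholder with a restore amount.
; Items named "Еда" (Food) show ResSatiety and all others show ResHitPoints; the use logic itself is not in this graph.
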(event EventBeginPlay
  (bind _objectwidgetcomponentnameanddescription (Variables|Default|GetObjectWidgetComponentNameAndDescription)
    (:then
      (bind _asw_object_items (Utilities|Casting|CastToW_Object_items (UserInterface|GetWidget _objectwidgetcomponentnameanddescription))
        (:then
          (Rendering|Components|TextRender|SetText (Variables|/Game/Object_items_Blueprints/W_Object_items.W_Object_items_C|GetNameObject _asw_object_items) (Utilities|Text|ToText(String) (Variables|Default|GetNameObject)))
          (if (Utilities|Enum|Equal(Enum) (Variables|Default|GetNameObject) "Еда")
            (Rendering|Components|TextRender|SetText (Variables|/Game/Object_items_Blueprints/W_Object_items.W_Object_items_C|GetDescriptionObject _asw_object_items) (Utilities|Text|ToText(String) (Utilities|String|Replace (Variables|Default|GetDescriptionObject) "#N#" (Utilities|String|ToString(Integer) (Variables|Default|GetResSatiety)))))
            (else
              (Rendering|Components|TextRender|SetText (Variables|/Game/Object_items_Blueprints/W_Object_items.W_Object_items_C|GetDescriptionObject _asw_object_items) (Utilities|Text|ToText(String) (Utilities|String|Replace (Variables|Default|GetDescriptionObject) "#N#" (Utilities|String|ToString(Integer) (Variables|Default|GetResHitPoints))))))))
        (:CastFailed
          (Development|PrintString "Hello"))))
    (:else)))

(event Collision|EventActorBeginOverlap
  (params (OtherActor :type Actor%20Object%20Reference)))

(event EventTick
  (params (DeltaSeconds :type Float%20%28single-precision%29)))

(fn ConstructionScript)