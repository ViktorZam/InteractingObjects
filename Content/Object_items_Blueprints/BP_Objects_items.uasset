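; Item actor that displays a name and description on a widget component alongside its static mesh.
; The construction script casts the widget to W_Object_items and fills its two text fields from NameObject and DescriptionObject.
; The SaveNameAndDescription event applies the same text through the component's user widget object.
; Disconnected construction-script nodes hold unused experiments in repositioning and scaling the widget with the mesh.
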(event Custom|SaveNameAndDescription
  (bind _asw_object_items (Utilities|Casting|CastToW_Object_items (UserInterface|GetUserWidgetObject (Variables|Default|GetObjectWidgetComponentNameAndDescription))))
  (Rendering|Components|TextRender|SetText (Variables|/Game/Object_items_Blueprints/W_Object_items.W_Object_items_C|GetNameObject _asw_object_items) (Utilities|Text|ToText(String) (Variables|Default|GetNameObject)))
  (Rendering|Components|TextRender|SetText (Variables|/Game/Object_items_Blueprints/W_Object_items.W_Object_items_C|GetDescriptionObject _asw_object_items) (Utilities|Text|ToText(String) (Variables|Default|GetDescriptionObject))))

(event EventBeginPlay)

(event Collision|EventActorBeginOverlap
  (params (OtherActor :type Actor%20Object%20Reference)))

(event EventTick
  (params (DeltaSeconds :type Float%20%28single-precision%29)))

(fn ConstructionScript
  (bind _asw_object_items (Utilities|Casting|CastToW_Object_items (UserInterface|GetWidget (Variables|Default|GetObjectWidgetComponentNameAndDescription))))
  (Rendering|Components|TextRender|SetText (Variables|/Game/Object_items_Blueprints/W_Object_items.W_Object_items_C|GetNameObject _asw_object_items) (Utilities|Text|ToText(String) (Variables|Default|GetNameObject)))
  (Rendering|Components|TextRender|SetText (Variables|/Game/Object_items_Blueprints/W_Object_items.W_Object_items_C|GetDescriptionObject _asw_object_items) (Utilities|Text|ToText(String) (Variables|Default|GetDescriptionObject))))